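; Game instance that handles hosting and joining multiplayer sessions.
; HOST_SESSION creates a session from a connection count and LAN flag, then opens the "New" level as a listen server.
; JOIN_SESSION joins a given search result, then locally spawns a NewController and a PrototypeShip at a fixed transform and has the controller possess the ship.
; Both events print their success or failure to screen.
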(event Custom|JOIN_SESSION
  (params (SearchResult :type Blueprint%20Session%20Result%20Structure%20%28by%20ref%29))
  (bind _returnvalue (Math|Transform|MakeTransform "0.000000, 0,200.000000"))
  (|JoinSession (Game|GetPlayerController 0) SearchResult
    (:OnSuccess
      (Development|PrintString "Successfully Joined")
      (bind _returnvalue_2 (Game|SpawnActorfromClass "/Game/newController.newController_C" _returnvalue "Undefined" 0 0))
      (bind _returnvalue_3 (Game|SpawnActorfromClass "/Game/PrototypeShip.PrototypeShip_C" _returnvalue "AdjustIfPossibleButDontSpawnIfColliding" 0 0))
      (Pawn|Possess _returnvalue_2 _returnvalue_3))
    (:OnFailure
      (Development|PrintString "Successfully Failed to Join"))))

(event Custom|HOST_SESSION
  (params (PublicConnections :type Integer) (bUseLAN :type Boolean))
  (|Session (Game|GetPlayerController 0) PublicConnections bUseLAN
    (:OnSuccess
      (Development|PrintString "Successfully Created")
      (Game|OpenLevel(byName) "New" true "listen"))
    (:OnFailure
      (Development|PrintString "Successfully Failed to Create"))))